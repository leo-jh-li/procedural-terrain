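; Procedural terrain actor that builds a height-mapped, vertex-coloured grid mesh in its construction script.
; GenerateMesh clears old data, gets an octave-based noise map from GenerateNoiseMap, then lays out vertices around the actor with Z scaled by the noise.
; Each vertex takes the colour of the first Regions entry at or above its noise height.
; Two triangles per grid cell feed one procedural mesh section with the terrain material applied.
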(event `self.ReceiveBeginPlay`)

(fn `[GetPerlinNoise]`
  (params (X :type "Float (double-precision)") (Y :type "Float (double-precision)") (Scale :type "Float (double-precision)"))
  (returns (Noise :type "Float (double-precision)"))
  (locals (LocalScale :type "Float (double-precision)"))
  (bind _returnvalue (`PerlinNoise2D.PerlinNoise2D` X Y Scale))
  (`KismetSystemLibrary.PrintString` (`KismetStringLibrary.Conv_DoubleToString` _returnvalue))
  (return _returnvalue))

(fn `ClearMesh`
  (`KismetArrayLibrary.Array_Clear` (`self.Vertices`))
  (`KismetArrayLibrary.Array_Clear` (`self.Triangles`))
  (`KismetArrayLibrary.Array_Clear` (`self.NoiseMap`))
  (`KismetArrayLibrary.Array_Clear` (`self.Colours`)))

(fn `GenerateMesh`
  (params (Rows :type Integer) (Columns :type Integer) (`Noise Scale` :type "Float (double-precision)") (Octaves :type Integer) (Persistence :type "Float (double-precision)") (Launcarity :type "Float (double-precision)") (HeightMultiplier :type "Float (double-precision)") (TriangleWidth :type "Float (double-precision)") (TriangleHeight :type "Float (double-precision)"))
  (set `self.Rows` Rows)
  (set `self.Columns` Columns)
  (set `self.NoiseScale` `Noise Scale`)
  (set `self.Octaves` Octaves)
  (set `self.Persistence` Persistence)
  (set `self.Lacunarity` Launcarity)
  (set `self.HeightMultiplier` HeightMultiplier)
  (set `self.TriangleWidth` TriangleWidth)
  (set `self.TriangleHeight` TriangleHeight)
  (`self.ClearMesh`)
  (set `self.NoiseMap` (`GenerateNoiseMap.GenerateNoiseMap` (`self.Rows`) (`self.Columns`) (`self.NoiseScale`) (`self.Octaves`) (`self.Persistence`) (`self.Lacunarity`) (`self.HeightWeight`)))
  ;[1 1 1] Create Rows × Columns vertices
  (set `self.StartLocation` (`KismetMathLibrary.MakeVector` (- 0.0 (/ (* (`KismetMathLibrary.Conv_IntToDouble` (- (`self.Columns`) 1)) (`self.TriangleHeight`)) 2.0)) (- 0.0 (/ (* (`KismetMathLibrary.Conv_IntToDouble` (- (`self.Rows`) 1)) (`self.TriangleWidth`)) 2.0)) (.z (`self.K2_GetActorLocation`)))) ; Centre mesh on parent
  (set `self.CurrVertex` (`self.StartLocation`)) ; Initialize first vertex
  (for _index (range (* (`self.Rows`) (`self.Columns`)))
    (bind _output (`|GetArrayItem` (`self.NoiseMap`) _index))
    (`KismetArrayLibrary.Array_Add` (`self.Vertices`) (`KismetMathLibrary.MakeVector` (.x (`self.CurrVertex`)) (.y (`self.CurrVertex`)) (+ (.z (`self.StartLocation`)) (* (`self.HeightMultiplier`) _output))))
    (bind _colour (`self.GetColourFromHeight` _output)) ; Add this vertex's colour into the colour map
    (`KismetArrayLibrary.Array_Add` (`self.Colours`) _colour)
    (if (== (mod (+ _index 1) (`self.Columns`)) 0)
      (set `self.CurrVertex` (`KismetMathLibrary.MakeVector` (.x (`self.StartLocation`)) (+ (`self.TriangleHeight`) (.y (`self.CurrVertex`))) (.z (`self.CurrVertex`)))) ; Reset vertex position's x and increment y by TriangleHeight
      (else
        (set `self.CurrVertex` (`KismetMathLibrary.MakeVector` (+ (`self.TriangleWidth`) (.x (`self.CurrVertex`))) (.y (`self.CurrVertex`)) (.z (`self.CurrVertex`)))) ; Increment vertex position's x by TriangleWidth
      )))
  ;[1 1 1] Specify triangles
  (for _index_2 (range (* (- (`self.Rows`) 1) (`self.Columns`)))
    (if (not (== (mod (+ _index_2 1) (`self.Columns`)) 0))
      ;;[1 1 1] Insert first triangle of this vertex into Triangles array
      (`KismetArrayLibrary.Array_Add` (`self.Triangles`) _index_2)
      (`KismetArrayLibrary.Array_Add` (`self.Triangles`) (+ _index_2 (`self.Columns`)))
      (`KismetArrayLibrary.Array_Add` (`self.Triangles`) (+ _index_2 1))
      ;;[1 1 1] Insert other triangle of this vertex
      (`KismetArrayLibrary.Array_Add` (`self.Triangles`) (+ _index_2 (`self.Columns`) 1))
      (`KismetArrayLibrary.Array_Add` (`self.Triangles`) (+ _index_2 1))
      (`KismetArrayLibrary.Array_Add` (`self.Triangles`) (+ _index_2 (`self.Columns`)))))
  (`ProceduralMeshComponent.CreateMeshSection_LinearColor` :`self` (`self.ProceduralMesh`) :`Vertices` (`self.Vertices`) :`Triangles` (`self.Triangles`) :`VertexColors` (`self.Colours`))
  (`PrimitiveComponent.SetMaterial` (`self.ProceduralMesh`) 0 "/Game/TerrainMaterial.TerrainMaterial"))

(fn `GetColourFromHeight`
  (params (Height :type "Float (double-precision)"))
  (returns (Colour :type "LinearColor Structure"))
  (locals (Regions :type "Array of /Game/Region Structure"))
  (for _array_element (`local.Regions`)
    (if (<= Height (`.Height_10_3A1B02E1462B9202E1209083BAA2C4C1` (break `/Game/Region` _array_element)))
      (return (`.Colour_12_E5EDFC04486BA7447EAA72B1A7230CEB` (break `/Game/Region` _array_element))))))

(fn `UserConstructionScript`
  (`self.GenerateMesh` (`self.Rows`) (`self.Columns`) (`self.NoiseScale`) (`self.Octaves`) (`self.Persistence`) (`self.Lacunarity`) (`self.HeightMultiplier`) (`self.TriangleWidth`) (`self.TriangleHeight`)))