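; MoveableCameraChar is a camera character that hosts a settings HUD for the player.
; On BeginPlay it creates the HUD widget, adds it to the viewport, shows the cursor, and sets permanent mouse capture with locked Game and UI input.
; Pressing G flips a visibility flag that shows or collapses the HUD.
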(event `self.ReceiveBeginPlay`
  (bind _returnvalue (`GameplayStatics.GetPlayerController` 0))
  (bind _returnvalue_2 (`|CreateWidget` "/Game/Blueprints/GenSettingsHUD.GenSettingsHUD_C"))
  (bind _output_get (set `self.HUDReference` _returnvalue_2))
  (`UserWidget.AddToViewport` _output_get 0)
  (`GameplayStatics.SetViewportMouseCaptureMode` "CapturePermanently")
  (set `PlayerController.bShowMouseCursor` true _returnvalue)
  (`WidgetBlueprintLibrary.SetInputMode_GameAndUIEx` _returnvalue null "LockAlways"))

(event `Key|G`
  (params (Key :type "Key Structure"))
  (bind _hudreference (`self.HUDReference`))
  (:`Pressed`
    (bind _output_get (set `self.HUDVisible` (not (`self.HUDVisible`))))
    (if _output_get
      (`Widget.SetVisibility` _hudreference "Visible")
      (else
        (`Widget.SetVisibility` _hudreference "Collapsed")))))

(fn `UserConstructionScript`)